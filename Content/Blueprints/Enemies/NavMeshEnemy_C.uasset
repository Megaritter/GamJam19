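; NavMeshEnemy is an enemy that moves to a target location on BeginPlay through a simple controller move, with a hover effect driven by its spring arm.
; Timeline_0 varies the arm length above a base height that the construction script also sets.
; Each of its updates calls Play on Timeline_1, which sways the arm's target offset along X only; the Y track's scaled value is unused.
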(event `self.ReceiveBeginPlay`
  (`NavigationSystem.SimpleMoveToLocation` (`self.GetController`) (`self.TargetLocation`))
  (bind (_direction _newtrack_0) (`Timeline|Timeline_0`)
    (:`Update`
      (set `SpringArmComponent.TargetArmLength` (+ (* _newtrack_0 (`self.HoverMaxZOffset`)) (`self.HoverBase`)) (`self.SpringArm`))
      (bind (_direction_2 _x _y) (`Timeline|Timeline_1`)
        (:`Update`
          (set `SpringArmComponent.TargetOffset` (`KismetMathLibrary.MakeVector` (* _x (`self.HoverMaxXYOffset`))) (`self.SpringArm`)))))))

(fn `UserConstructionScript`
  (set `SpringArmComponent.TargetArmLength` (`self.HoverBase`) (`self.SpringArm`)))
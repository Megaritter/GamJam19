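; Behavior tree decorator for enemy AI that gates a branch on the pawn's distance to a blackboard target location.
; It casts the owner to EnemyAIController, stores that reference, and measures from the controlled pawn to the TargetLocationKey vector.
; Despite the CloseEnough name, the condition passes when that distance is at least AcceptableDistance, so it is true while the pawn is still far away.
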(fn `PerformConditionCheck`
  (params (OwnerActor :type "Actor Object Reference"))
  (returns (ReturnValue :type Boolean))
  (bind _asenemy_aicontroller (cast `/Game/Blueprints/Enemies/EnemyAIController` OwnerActor))
  (set `self.AIConRef` _asenemy_aicontroller)
  (return (>= (`KismetMathLibrary.VSize` (- (`BTFunctionLibrary.GetBlackboardValueAsVector` (`self.TargetLocationKey`)) (`Actor.K2_GetActorLocation` (`Controller.K2_GetPawn` (`self.AIConRef`))))) (`self.AcceptableDistance`))))
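; Enemy actor whose transform is set externally along a spline and that fires arrow projectiles at objects in front of it.
; Each tick, unless reloading, it line-traces along its mesh's forward vector; a hit spawns and launches an Arrow offset along the right vector, then starts a reload timer.
; Damage reduces Health, and at zero it notifies its spline spawner reference and destroys itself.
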(event `self.ReceiveTick`
  (params (DeltaSeconds :type "Float (single-precision)"))
  (bind _staticmesh1 (`self.StaticMesh1`))
  (bind _returnvalue (`SceneComponent.K2_GetComponentLocation` _staticmesh1))
  (if (not (`self.bHasToReload?`))
    (bind (_outhit _returnvalue_2) (`KismetSystemLibrary.LineTraceSingleForObjects` :`Start` _returnvalue :`End` (+ _returnvalue (* (`SceneComponent.GetForwardVector` _staticmesh1) 10000.0)) :`ObjectTypes` (`self.ObjectsToScanFor`) :`DrawDebugType` "ForOneFrame"))
    (if _returnvalue_2
      (`self.ShootProjectile`))))

(event `SetPosOnSpline`
  (params (NewParam :type "Transform Structure"))
  (`SceneComponent.K2_SetWorldTransform` (`self.DefaultSceneRoot`) NewParam false false))

(event `self.ReceiveAnyDamage`
  (params (Damage :type "Float (single-precision)") (DamageType :type "DamageType Object Reference") (InstigatedBy :type "Controller Object Reference") (DamageCauser :type "Actor Object Reference"))
  (bind _output_get (set `self.Health` (- (`self.Health`) Damage)))
  (if (<= _output_get 0.0)
    (if (not (`self.IsActorBeingDestroyed`))
      (`self.OnDeath`))))

(event `ShootProjectile`
  (bind _staticmesh1 (`self.StaticMesh1`))
  (bind (_returnvalue_location _returnvalue_rotation) (`KismetMathLibrary.BreakTransform` (`SceneComponent.K2_GetComponentToWorld` _staticmesh1)))
  (bind _returnvalue (`|SpawnActorFromClass` "/Game/Blueprints/Bogen/Arrow.Arrow_C" (`KismetMathLibrary.MakeTransform` (+ _returnvalue_location (* (`SceneComponent.GetRightVector` _staticmesh1) 500.0)) _returnvalue_rotation) "Undefined" "OverrideRootScale" null null))
  (`/Game/Blueprints/Bogen/Arrow.ShootEvent` _returnvalue 10000.0)
  (set `self.bHasToReload?` true)
  (`KismetSystemLibrary.K2_SetTimerDelegate` (delegate `Reload`) (`self.ReloadTime`)))

(event `Reload`
  (set `self.bHasToReload?` false))

(fn `OnDeath`
  (`/Game/Blueprints/Enemies/SplineEnemySpawn_A.OnEnemyActorDestroyed` (`self.SplineSpawnRef`))
  (`self.K2_DestroyActor`))

(fn `UserConstructionScript`)
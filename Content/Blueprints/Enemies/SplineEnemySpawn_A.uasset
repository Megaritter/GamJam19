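; Enemy spawner actor that spawns an enemy, moves it along an approach spline and then repeatedly around a loop spline.
; Timelines, played only when not occupied, drive the enemy's SetPosOnSpline with transforms sampled along each spline.
; The Construction Script derives play rates from durations and snaps the loop spline to the approach's end.
; OnEnemyActorDestroyed stops both timelines and respawns after a delay.
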(event `OnEnemyActorDestroyed`
  (bind (_returnvalue_location _returnvalue_rotation) (`KismetMathLibrary.BreakTransform` (`SceneComponent.K2_GetComponentToWorld` (`self.DefaultSceneRoot`))))
  (`self.InterruptTimelineApproach`)
  (`self.InterruptTimelineLoop`)
  (`KismetSystemLibrary.Delay` (`self.RespawnDelay`))
  (bind _returnvalue (`|SpawnActorFromClass` (`self.EnemyClass`) (`KismetMathLibrary.MakeTransform` _returnvalue_location _returnvalue_rotation) "AlwaysSpawn" "OverrideRootScale" null 0.1 null :!label _label))
  (set `/Game/Blueprints/Enemies/SplineEnemy_Actor.SplineSpawnRef` self _returnvalue)
  (set `self.EnemyActor` _returnvalue)
  (if (not (`self.bIsOccupied?`))
    (bind (_direction _position) (`Timeline|TimeLineApproach` :`NewTime` 0.0 :!via `PlayFromStart` :!label _label_2)
      (:`Update`
        (bind _transform (`self.GetTransformOnSpine` (`self.SplineApproach`) _position))
        (`/Game/Blueprints/Enemies/SplineEnemy_Actor.SetPosOnSpline` (`self.EnemyActor`) _transform))
      (:`Finished`
        (bind (_direction_2 _newtrack_1) (`Timeline|TimeLineLoop` :!via `PlayFromStart` :!label _label_3)
          (:`Update`
            (bind _transform_2 (`self.GetTransformOnSpine` (`self.SplineLoop`) _newtrack_1))
            (`/Game/Blueprints/Enemies/SplineEnemy_Actor.SetPosOnSpline` (`self.EnemyActor`) _transform_2))
          (:`Finished`
            (`KismetSystemLibrary.Delay` 0.1)
            (goto _label_3 :!via `PlayFromStart`)))))))

(event `self.ReceiveBeginPlay`
  (goto _label))

(event `InterruptTimelineApproach`
  (goto _label_2 :!via `Stop`))

(event `InterruptTimelineLoop`
  (goto _label_3 :!via `Stop`))

(fn `GetTransformOnSpine`
  (params (Spline :type "SplineComponent Object Reference") (TimelineValue :type "Float (double-precision)"))
  (returns (Transform :type "Transform Structure"))
  (bind _returnvalue (* (`SplineComponent.GetSplineLength` Spline) TimelineValue))
  (return (`KismetMathLibrary.MakeTransform` (`SplineComponent.GetLocationAtDistanceAlongSpline` Spline _returnvalue "World") (`SplineComponent.GetRotationAtDistanceAlongSpline` Spline _returnvalue "World") (`SceneComponent.K2_GetComponentScale` (`/Game/Blueprints/Enemies/SplineEnemy_Actor.DefaultSceneRoot` (`self.EnemyActor`))))))

(fn `UserConstructionScript`
  (bind _splineapproach (`self.SplineApproach`))
  (`TimelineComponent.SetPlayRate` (`self.TimeLineApproach`) (/ 1.0 (`self.DurationApproach`)))
  (`TimelineComponent.SetPlayRate` (`self.TimeLineLoop`) (/ 1.0 (`self.DurationLoop`)))
  (`SceneComponent.K2_SetWorldLocation` (`self.SplineLoop`) (`SplineComponent.GetLocationAtDistanceAlongSpline` _splineapproach (`SplineComponent.GetSplineLength` _splineapproach) "World") false false))
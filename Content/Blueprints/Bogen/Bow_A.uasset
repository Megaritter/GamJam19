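; Bow actor drawn with two motion controllers that spawns an Anker_A actor on its skeletal mesh at BeginPlay.
; While drawing, Tick feeds right-hand distance over MaxDraw into the anim blueprint's DrawPercentage.
; Bow rotation takes roll from the left controller, pitch and yaw from the right.
; Release stops drawing and releases the anchor, also firing automatically when that draw ratio exceeds MaxDraw.
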(event `self.ReceiveBeginPlay`
  (bind _skeletalmesh (`self.SkeletalMesh`))
  (bind _returnvalue (`|SpawnActorFromClass` "/Game/Blueprints/Bogen/Anker_A.Anker_A_C" (`KismetMathLibrary.MakeTransform` (`SceneComponent.GetSocketLocation` _skeletalmesh "AnkerSocket") (`self.K2_GetActorRotation`)) "Undefined" "OverrideRootScale" null null))
  (`self.K2_AttachToComponent` _returnvalue _skeletalmesh "Bone_024" "SnapToTarget" "SnapToTarget" "KeepWorld" true)
  (set `self.AnkerRef` _returnvalue)
  (set `/Game/Blueprints/Bogen/Anker_A.OwningBow` self _returnvalue)
  (`KismetSystemLibrary.PrintString` "Anker Spawned and attached"))

(event `StartDraw`
  (`KismetSystemLibrary.PrintString` "Start Draw in Bow")
  (set `self.bIsDrawing?` true))

(event `Release`
  (set `self.bIsDrawing?` false)
  (`/Game/Blueprints/Bogen/Anker_A.Release` (`self.AnkerRef`)))

(event `self.ReceiveTick`
  (params (DeltaSeconds :type "Float (single-precision)"))
  (bind _returnvalue_roll (`KismetMathLibrary.BreakRotator` (`SceneComponent.K2_GetComponentRotation` (`/Game/Blueprints/VRPlayer/BP_MotionController.MotionController` (`self.LeftHandController`)))))
  (bind (_returnvalue_roll_2 _returnvalue_pitch _returnvalue_yaw) (`KismetMathLibrary.BreakRotator` (`SceneComponent.K2_GetComponentRotation` (`/Game/Blueprints/VRPlayer/BP_MotionController.MotionController` (`self.RightHandController`)))))
  (if (`self.bIsDrawing?`)
    (`KismetSystemLibrary.PrintString` (`KismetStringLibrary.Concat_StrStr` "Draw on Bow_A: " (`KismetStringLibrary.Conv_DoubleToString` (`self.CalculateDrawInPercentage`))))
    ;[1 1 1] Bow Rotation and Draw
    (bind _asbogen_v_04_skeleton_anim_blueprint (cast `/Game/VirtualRealityBP/Blueprints/Bogen_v04_Skeleton_AnimBlueprint` (`SkeletalMeshComponent.GetAnimInstance` (`self.SkeletalMesh`))))
    (set `/Game/VirtualRealityBP/Blueprints/Bogen_v04_Skeleton_AnimBlueprint.DrawPercentage` (`self.CalculateDrawInPercentage`) _asbogen_v_04_skeleton_anim_blueprint)
    (`self.K2_SetActorRotation` self (`KismetMathLibrary.MakeRotator` _returnvalue_roll _returnvalue_pitch _returnvalue_yaw) false)
    (if (> (`self.CalculateDrawInPercentage`) (`self.MaxDraw`))
      (`self.Release`))))

(fn `CalculateDrawInPercentage`
  (returns (Draw :type "Float (double-precision)"))
  (return (/ (`KismetMathLibrary.VSize` (- (`self.K2_GetActorLocation`) (`SceneComponent.K2_GetComponentLocation` (`/Game/Blueprints/VRPlayer/BP_MotionController.MotionController` (`self.RightHandController`))))) (`self.MaxDraw`))))

(fn `UserConstructionScript`)
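; Quiver actor for VR bow play that hands a new arrow to a motion controller reaching into its HitBox.
; On overlap, it proceeds only for a right-hand BP_MotionController whose AttachedArrow is already valid.
; It then spawns an Arrow at the overlapping component, snaps it to ArrowSocket and overwrites the controller's AttachedArrow reference with it.
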(event `self.HitBox.OnComponentBeginOverlap`
  (params (OverlappedComponent :type "PrimitiveComponent Object Reference") (OtherActor :type "Actor Object Reference") (OtherComp :type "PrimitiveComponent Object Reference") (OtherBodyIndex :type Integer) (bFromSweep :type Boolean) (SweepResult :type "HitResult Structure (by ref)"))
  (bind _asbp_motion_controller (cast `/Game/Blueprints/VRPlayer/BP_MotionController` OtherActor))
  (if (and (`|EnumEquality` (`/Game/Blueprints/VRPlayer/BP_MotionController.Hand` _asbp_motion_controller) "Right") (`KismetSystemLibrary.IsValid` (`/Game/Blueprints/VRPlayer/BP_MotionController.AttachedArrow` _asbp_motion_controller)))
    (bind _returnvalue (`|SpawnActorFromClass` "/Game/Blueprints/Bogen/Arrow.Arrow_C" (`SceneComponent.K2_GetComponentToWorld` OtherComp) "Undefined" "OverrideRootScale" null null))
    (`self.K2_AttachToComponent` _returnvalue OtherComp "ArrowSocket" "SnapToTarget" "KeepRelative" "KeepRelative" true)
    (set `/Game/Blueprints/VRPlayer/BP_MotionController.AttachedArrow` _returnvalue _asbp_motion_controller)))

(fn `UserConstructionScript`)